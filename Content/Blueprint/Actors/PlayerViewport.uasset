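; Player camera for a mouse-driven view that pans, zooms by FOV and flies into clickable locations of interest.
; ZoomIn hides all locations, then a timeline blends camera transform and FOV under a fade widget and whoosh, ending with the location's people and a BackOut widget.
; ZoomOut reverses that timeline and unhides the locations.
; Panning is blocked while zoomed or lerping, and re-caches the camera's return transform on each move.
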(event `self.ReceiveBeginPlay`
  (bind _returnvalue (`GameplayStatics.GetPlayerController` 0))
  (set `PlayerController.bShowMouseCursor` true _returnvalue)
  (set `PlayerController.bEnableClickEvents` true _returnvalue)
  (set `self.OriginalCameraTransform` (`SceneComponent.K2_GetComponentToWorld` (`self.Camera`)))
  (`EnhancedInputSubsystemInterface.AddMappingContext` (pcsubsystem `EnhancedInputLocalPlayerSubsystem` (`GameplayStatics.GetPlayerController` 0)) "/Game/Inputs/NewInputMappingContext.NewInputMappingContext" 0 (struct)))

(event `ZoomIn`
  (params (NewParam :type "Transform Structure") (NewParam2 :type "/Game/Blueprint/Actors/LocationOfInterest Object Reference"))
  (bind _camera (`self.Camera`))
  (set `self.New Transform` NewParam)
  (set `self.ZoomedIn` true)
  (set `self.location of interest` NewParam2)
  (set `self.lerping` true)
  (bind _outactors (`GameplayStatics.GetAllActorsOfClass` "/Game/Blueprint/Actors/LocationOfInterest.LocationOfInterest_C"))
  (for _array_element _outactors
    (`self.SetActorHiddenInGame` _array_element (`self.ZoomedIn`)))
  (`self.FadeInOut`)
  (`GameplayStatics.PlaySound2D` "/Game/Sound/WooshUpdated.WooshUpdated" 1.0 1.0 0.0 null null)
  (bind (_direction _newtrack_1 _zoom) (`Timeline|Move to` :!label _label)
    (:`Update`
      (`self.LerpTrnaform` _newtrack_1)
      (`CameraComponent.SetFieldOfView` _camera (`KismetMathLibrary.Lerp` (`CameraComponent.FieldOfView` _camera) 90.0 _zoom)))
    (:`Finished`
      (`self.SetVisibility`)
      (if (`self.ZoomedIn`)
        (bind _returnvalue (`|CreateWidget` "/Game/Blueprint/Widgets/BackOut.BackOut_C" (`GameplayStatics.GetPlayerController` 0)))
        (`UserWidget.AddToViewport` _returnvalue 0)
        (`KismetSystemLibrary.Delay` 1.0)
        (set `self.lerping` false)))))

(event `ZoomOut`
  (set `self.ZoomedIn` false)
  (`self.ZoomOutDis`)
  (set `self.lerping` true)
  (`self.FadeInOut`)
  (`GameplayStatics.PlaySound2D` "/Game/Sound/WooshUpdated.WooshUpdated" 1.0 1.0 0.0 null null)
  (goto _label :!via `Reverse`))

(event `EnhancedInput|/Game/Inputs/IA_MoveUpDown`
  (params (ActionValue :type "Float (double-precision)") (ElapsedSeconds :type "Float (double-precision)") (TriggeredSeconds :type "Float (double-precision)") (InputAction :type "InputAction Object Reference" :default "/Game/Inputs/IA_MoveUpDown.IA_MoveUpDown"))
  (:`Triggered`
    (if (and (not (`self.ZoomedIn`)) (not (`self.lerping`)))
      (`self.Move` (`KismetMathLibrary.MakeVector` (* ActionValue 20.0))))))

(event `FadeInOut`
  (bind _returnvalue (`|CreateWidget` "/Game/Blueprint/Widgets/FadeInAndOut.FadeInAndOut_C" (`GameplayStatics.GetPlayerController` 0)))
  (`UserWidget.AddToViewport` _returnvalue 100))

(event `EnhancedInput|/Game/Inputs/IA_MoveRightLEft`
  (params (ActionValue :type "Float (double-precision)") (ElapsedSeconds :type "Float (double-precision)") (TriggeredSeconds :type "Float (double-precision)") (InputAction :type "InputAction Object Reference" :default "/Game/Inputs/IA_MoveRightLEft.IA_MoveRightLEft"))
  (:`Triggered`
    (if (and (not (`self.ZoomedIn`)) (not (`self.lerping`)))
      (`self.Move` (`KismetMathLibrary.MakeVector` 0.0 (* ActionValue 20.0))))))

(event `EnhancedInput|/Game/Inputs/IA_ZoomInOut`
  (params (ActionValue :type "Float (double-precision)") (ElapsedSeconds :type "Float (double-precision)") (TriggeredSeconds :type "Float (double-precision)") (InputAction :type "InputAction Object Reference" :default "/Game/Inputs/IA_ZoomInOut.IA_ZoomInOut"))
  (bind _camera (`self.Camera`))
  (:`Triggered`
    (if (not (`self.question`))
      (`CameraComponent.SetFieldOfView` _camera (`KismetMathLibrary.FClamp` (+ (`CameraComponent.FieldOfView` _camera) (* ActionValue -5.0)) 30.0 100.0)))))

(fn `LerpTrnaform`
  (params (Alpha :type "Float (single-precision)"))
  (`SceneComponent.K2_SetWorldTransform` (`self.Camera`) (`KismetMathLibrary.TLerp` (`self.OriginalCameraTransform`) (`self.New Transform`) Alpha) false false))

(fn `Move`
  (params (DeltaLocation :type "Vector Structure"))
  (`self.K2_AddActorWorldOffset` DeltaLocation true)
  (set `self.OriginalCameraTransform` (`SceneComponent.K2_GetComponentToWorld` (`self.Camera`))))

(fn `SetVisibility`
  (bind _zoomedin (`self.ZoomedIn`))
  (set `self.lerping` false)
  (if _zoomedin
    (`/Game/Blueprint/Actors/LocationOfInterest.HidePeople` (`self.location of interest`) false)
    (else
      (bind _outactors (`GameplayStatics.GetAllActorsOfClass` "/Game/Blueprint/Actors/LocationOfInterest.LocationOfInterest_C"))
      (for _array_element _outactors
        (`self.SetActorHiddenInGame` _array_element _zoomedin)))))

(fn `UserConstructionScript`)