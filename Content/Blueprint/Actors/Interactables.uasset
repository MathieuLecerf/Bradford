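; Interactables is a clickable quiz or info actor that shows a portrait on a plane matched to the player's rotation.
; Clicking it opens its QuestionType widget, passing the question and itself, and flags the player viewport as busy.
; Integer or case-insensitive text checks play feedback sounds; correct answers update the game mode's bar, hide the actor and unbind clicks.
; Finished info dumps also update the bar, and InfoDump and Dialogue types can reappear after completion.
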(event `Should i be Visible`
  (params (`Hidden in Game` :type Boolean))
  (bind _question_portrait (break `/Game/DataTables/QuestionStructure` (`self.Question`)))
  (bind _questiontype (`self.QuestionType`))
  (if (or (== _questiontype "/Game/Blueprint/Widgets/InfoDump.InfoDump_C") (== _questiontype "/Game/Blueprint/Widgets/Dialogue.Dialogue_C"))
    (`self.SetActorHiddenInGame` `Hidden in Game`)
    (elif (`self.Answer Correct`)
      (`self.SetActorHiddenInGame` true)
      (else
        (`self.SetActorHiddenInGame` `Hidden in Game`))))
  (bind _asplayer_viewport (cast `/Game/Blueprint/Actors/PlayerViewport` (`GameplayStatics.GetPlayerPawn` 0)))
  (`SceneComponent.K2_SetWorldRotation` (`self.Plane`) (`self.K2_GetActorRotation` _asplayer_viewport) false false)
  (bind _returnvalue (`PrimitiveComponent.CreateDynamicMaterialInstance` (`self.Plane`) 0 "/Game/Blueprint/Actors/BaseTexture.BaseTexture" "None"))
  (`PrimitiveComponent.SetMaterial` (`self.Plane`) 0 _returnvalue)
  (bind _output_get (set `self.NewVar` _returnvalue))
  (`MaterialInstanceDynamic.SetTextureParameterValue` _output_get "PT" _question_portrait))

(event `self.ReceiveBeginPlay`
  (`self.SetActorHiddenInGame` true)
  (add `self.OnClicked` (delegate `OnClicked_Event`)))

(event `OnClicked_Event` :!signature `self.OnClicked`
  (params (TouchedActor :type "Actor Object Reference") (ButtonPressed :type "Key Structure" :default "None"))
  (bind _asplayer_viewport (cast `/Game/Blueprint/Actors/PlayerViewport` (`GameplayStatics.GetPlayerPawn` 0)))
  (if (`KismetMathLibrary.BooleanNOR` (`/Game/Blueprint/Actors/PlayerViewport.question` _asplayer_viewport) (`self.bHidden`))
    (bind _returnvalue (`|CreateWidget` (`self.QuestionType`) (`GameplayStatics.GetPlayerController` 0)))
    (`UserWidget.AddToViewport` _returnvalue 0)
    (set `/Game/Blueprint/Actors/PlayerViewport.question` true _asplayer_viewport)
    (bind _output_get (set `self.Widget` _returnvalue))
    (message `/Game/Blueprint/Interfaces/UI_Interface.STuff` _output_get (`self.Question`) self)))

(event `/Game/Blueprint/Interfaces/PersonInterface.Exit`
  (set `/Game/Blueprint/Actors/PlayerViewport.question` false (stale `OnClicked_Event` _asplayer_viewport)))

(event `/Game/Blueprint/Interfaces/PersonInterface.CheckAnswerInt`
  (params (Answer :type Integer))
  (bind (_question_portrait _question_blurb _question_answer1 _question_answer2 _question_answerr3 _question_answer4 _question_correctanswer) (break `/Game/DataTables/QuestionStructure` (`self.Question`)))
  (if (not (`self.Answer Correct`))
    (if (== Answer _question_correctanswer)
      (`KismetSystemLibrary.PrintString` "correct")
      (set `self.Answer Correct` true)
      (message `/Game/Blueprint/Interfaces/I_GameMode.UpdateBar` (`GameplayStatics.GetGameMode`))
      (`self.SetActorHiddenInGame` true)
      (clear `self.OnClicked`)
      (`GameplayStatics.PlaySound2D` "/Game/Sound/546084__stavsounds__correct.546084__stavsounds__correct" 1.0 1.0 0.0 null null)
      (message `/Game/Blueprint/Interfaces/UI_Interface.Correct` (`self.Widget`))
      (else
        (`KismetSystemLibrary.PrintString` "Incorrect")
        (set `self.Answer Correct` false)
        (`GameplayStatics.PlaySound2D` "/Game/Sound/529384__beetlemuse__invalid-selection.529384__beetlemuse__invalid-selection" 1.0 1.0 0.0 null null)))
    (else
      (`KismetSystemLibrary.PrintString` "already answered"))))

(event `/Game/Blueprint/Interfaces/PersonInterface.CheckAnswerText`
  (params (Answer :type Text))
  (bind (_question_portrait _question_blurb _question_answer1 _question_answer2 _question_answerr3 _question_answer4 _question_correctanswer _question_singleanswer) (break `/Game/DataTables/QuestionStructure` (`self.Question`)))
  (if (not (`self.Answer Correct`))
    (if (`KismetStringLibrary.EqualEqual_StrStr` (`KismetTextLibrary.Conv_TextToString` (`KismetTextLibrary.TextToLower` Answer)) (`KismetTextLibrary.Conv_TextToString` (`KismetTextLibrary.TextToLower` _question_singleanswer)))
      (`KismetSystemLibrary.PrintString` "correct")
      (set `self.Answer Correct` true)
      (message `/Game/Blueprint/Interfaces/I_GameMode.UpdateBar` (`GameplayStatics.GetGameMode`))
      (`self.SetActorHiddenInGame` true)
      (clear `self.OnClicked`)
      (`GameplayStatics.PlaySound2D` "/Game/Sound/546084__stavsounds__correct.546084__stavsounds__correct" 1.0 1.0 0.0 null null)
      (message `/Game/Blueprint/Interfaces/UI_Interface.Correct` (`self.Widget`))
      (else
        (`KismetSystemLibrary.PrintString` "Incorrect")
        (set `self.Answer Correct` false)
        (`GameplayStatics.PlaySound2D` "/Game/Sound/529384__beetlemuse__invalid-selection.529384__beetlemuse__invalid-selection" 1.0 1.0 0.0 null null)))))

(event `/Game/Blueprint/Interfaces/PersonInterface.EndInfoDump`
  (if (not (`self.Answer Correct`))
    (set `self.Answer Correct` true)
    (message `/Game/Blueprint/Interfaces/I_GameMode.UpdateBar` (`GameplayStatics.GetGameMode`))))

(fn `Set Questions`
  (params (Question :type "/Game/DataTables/QuestionStructure Structure"))
  (set `self.Question` Question))

(fn `UserConstructionScript`)