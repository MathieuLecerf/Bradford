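; LocationOfInterest is a clickable actor that sends the player's camera in to a point of interest until it is marked Complete.
; On BeginPlay it hides if complete, aligns its plane to the PlayerViewport pawn's rotation and applies TextureValue through a dynamic material.
; Clicking passes the Arrow transform, positioned by the construction script, to the pawn's ZoomIn.
; It also binds the pawn's zoom-out dispatcher to hide the linked People.
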(event `self.ReceiveBeginPlay`
  (add `self.OnClicked` (delegate `OnClicked_Event`))
  (`self.SetActorHiddenInGame` (`self.Complete`))
  (bind _asplayer_viewport (cast `/Game/Blueprint/Actors/PlayerViewport` (`GameplayStatics.GetPlayerPawn` 0)))
  (`SceneComponent.K2_SetWorldRotation` (`self.Plane`) (`self.K2_GetActorRotation` _asplayer_viewport) false false)
  (bind _returnvalue (`PrimitiveComponent.CreateDynamicMaterialInstance` (`self.Plane`) 0 "/Game/Blueprint/Actors/BaseTexture.BaseTexture" "None"))
  (`PrimitiveComponent.SetMaterial` (`self.Plane`) 0 _returnvalue)
  (bind _output_get (set `self.Material` _returnvalue))
  (`MaterialInstanceDynamic.SetTextureParameterValue` _output_get "PT" (`self.TextureValue`)))

(event `OnClicked_Event` :!signature `self.OnClicked`
  (params (TouchedActor :type "Actor Object Reference") (ButtonPressed :type "Key Structure" :default "None"))
  (if (not (`self.bHidden`))
    (if (`self.Complete`)
      (`self.SetActorHiddenInGame` true)
      (else
        (bind _asplayer_viewport (cast `/Game/Blueprint/Actors/PlayerViewport` (`GameplayStatics.GetPlayerPawn` 0)))
        (`/Game/Blueprint/Actors/PlayerViewport.ZoomIn` _asplayer_viewport (`SceneComponent.K2_GetComponentToWorld` (`self.Arrow`)) self)
        (add `/Game/Blueprint/Actors/PlayerViewport.ZoomOutDis` _asplayer_viewport (delegate `ZoomOutDis_Event`))))))

(event `ZoomOutDis_Event`
  (`self.HidePeople` true))

(fn `HidePeople`
  (params (bNewHidden :type Boolean))
  (for _array_element (`self.People`)
    (`/Game/Blueprint/Actors/Interactables.Should i be Visible` _array_element bNewHidden)))

(fn `UserConstructionScript`
  (`SceneComponent.K2_SetRelativeTransform` (`self.Arrow`) (`self.ArrowTrnsform`) false false))